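; BP_Unit is a movable character that walks along one of four world axis directions and shows its selection state through color.
; Every tick it feeds the vector chosen by InputDirection into CharacterMovement, plus a tiny constant +X nudge.
; SetInputDirection stores the direction and treats any value other than -1 as selected.
; SetSelected uses ChangeColor to darken one body part toward black, or restore BaseColor when deselected.
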(event `self.ReceiveTick`
  (params (DeltaSeconds :type "Float (single-precision)"))
  (bind _charactermovement (`self.CharacterMovement`))
  (`PawnMovementComponent.AddInputVector` _charactermovement (select `int` (`self.InputDirection`) :`0` (1.0 0.0 0.0) :`1` (0.0 1.0 0.0) :`2` (-1.0 0.0 0.0) :`3` (0.0 -1.0 0.0) :!type "Vector Structure") false)
  (`PawnMovementComponent.AddInputVector` _charactermovement (0.01 0.0 0.0) false))

(fn `SetInputDirection`
  (params (newInputDirection :type Integer))
  (bind _output_get (set `self.InputDirection` newInputDirection))
  (`self.SetSelected` (!= _output_get -1)))

(fn `SetSelected`
  (params (IsSelected :type Boolean))
  (if IsSelected
    (`self.ChangeColor` "NewEnumerator1" (`KismetMathLibrary.LinearColorLerp` (`self.BaseColor`) (struct) 0.9))
    (else
      (`self.ChangeColor` "NewEnumerator1" (`self.BaseColor`)))))

(fn `UserConstructionScript`)