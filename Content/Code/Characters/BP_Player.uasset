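; Player pawn that drives two spawned BP_Units, one green and one blue, from a single set of four directional inputs.
; An Input macro counts taps within TapThreshold: tap-and-hold steers the green unit, double-tap-and-hold the blue one.
; Releasing a direction clears it on whichever unit holds it.
; The pawn follows the units' midpoint each tick as the camera position, and ResetLevel reloads the current level.
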(event `InputAction|MoveLeft`
  (params (Key :type "Key Structure"))
  ;[0.315 0.651 0.1482] Check for movement events
  (:`Pressed`
    (`self.Input` (`self.TapNumberLeft`) (`self.TapHoldLeft`) :!label _label
      (:`Single`
        (`self.MovementPressedInput` 0 3))
      (:`Double`
        (`self.MovementPressedInput` 1 3))))
  (:`Released`
    (`self.MovementReleasedInput` 3)
    (goto _label :!via `Released`)))

(event `InputAction|MoveDown`
  (params (Key :type "Key Structure"))
  ;[0.315 0.651 0.1482] Check for movement events
  (:`Pressed`
    (`self.Input` (`self.TapNumberDown`) (`self.TapHoldDown`) :!label _label_2
      (:`Single`
        (`self.MovementPressedInput` 0 2))
      (:`Double`
        (`self.MovementPressedInput` 1 2))))
  (:`Released`
    (`self.MovementReleasedInput` 2)
    (goto _label_2 :!via `Released`)))

(event `InputAction|MoveRight`
  (params (Key :type "Key Structure"))
  ;[0.315 0.651 0.1482] Check for movement events
  (:`Pressed`
    (`self.Input` (`self.TapNumberRight`) (`self.TapHoldRight`) :!label _label_3
      (:`Single`
        (`self.MovementPressedInput` 0 1))
      (:`Double`
        (`self.MovementPressedInput` 1 1))))
  (:`Released`
    (`self.MovementReleasedInput` 1)
    (goto _label_3 :!via `Released`)))

(event `self.ReceiveTick`
  (params (DeltaSeconds :type "Float (single-precision)"))
  (bind _returnvalue (`self.K2_GetActorLocation` (`self.Player1`)))
  ;[0 0.1609 1] Set camera pos between players
  (`parent.ReceiveTick` DeltaSeconds)
  (`self.K2_SetActorLocation` (+ _returnvalue (* (- (`self.K2_GetActorLocation` (`self.Player0`)) _returnvalue) 0.5))))

(event `InputAction|ResetLevel`
  (params (Key :type "Key Structure"))
  ;[1 0 0] Movement Controls
  (:`Pressed`
    (bind _returnvalue (`GameplayStatics.GetCurrentLevelName` true))
    (`GameplayStatics.OpenLevel` (`KismetStringLibrary.Conv_StringToName` _returnvalue))))

(event `MovementPressedInput`
  (params (CharacterIndex :type Integer) (Direction :type Integer))
  ;[1 0 0] Movement Controls
  (`/Game/Code/Characters/BP_Unit.SetInputDirection` (select `int` CharacterIndex :`0` (`self.Player0`) :`1` (`self.Player1`)) Direction))

(event `InputAction|MoveUp`
  (params (Key :type "Key Structure"))
  ;[0.315 0.651 0.1482] Check for movement events
  (:`Pressed`
    (`self.Input` (`self.TapNumberUp`) (`self.TapHoldUp`) :!label _label_4
      (:`Single`
        (`self.MovementPressedInput` 0))
      (:`Double`
        (`self.MovementPressedInput` 1))))
  (:`Released`
    (`self.MovementReleasedInput` 0)
    (goto _label_4 :!via `Released`)))

(event `MovementReleasedInput`
  (params (Direction :type Integer))
  (bind _player0 (`self.Player0`))
  (bind _player1 (`self.Player1`))
  ;[1 0 0] Movement Controls
  (`|ExecutionSequence`
    (:`then_0`
      (if (== (`/Game/Code/Characters/BP_Unit.InputDirection` _player0) Direction)
        (`/Game/Code/Characters/BP_Unit.SetInputDirection` _player0 -1)))
    (:`then_1`
      (if (== Direction (`/Game/Code/Characters/BP_Unit.InputDirection` _player1))
        (`/Game/Code/Characters/BP_Unit.SetInputDirection` _player1 -1)))))

(event `self.ReceiveBeginPlay`
  (bind _returnvalue (`self.GetTransform`))
  (`|ExecutionSequence`
    (:`then_0`
      ;[1 0 0] Activate topdown camera
      (`ActorComponent.Activate` (`self.Camera`) false) ; actual activation
    )
    (:`then_1`
      ;[1 0.9764 0.1674] Spawn both units
      (bind _returnvalue_2 (`|SpawnActorFromClass` "/Game/Code/Characters/BP_Unit.BP_Unit_C" _returnvalue "Undefined" "OverrideRootScale" null null))
      (bind _output_get (set `self.Player0` _returnvalue_2))
      (bind _output_get_2 (set `/Game/Code/Characters/BP_Unit.BaseColor` (struct :`R` 0.202011 :`G` 0.776042 :`A` 1.0) _output_get))
      (`/Game/Base/BP_BaseCharacter.ChangeColor` _output_get "NewEnumerator1" _output_get_2))
    (:`then_2`
      (bind _returnvalue_3 (`|SpawnActorFromClass` "/Game/Code/Characters/BP_Unit.BP_Unit_C" _returnvalue "Undefined" "OverrideRootScale" null null))
      (bind _output_get_3 (set `self.Player1` _returnvalue_3))
      (bind _output_get_4 (set `/Game/Code/Characters/BP_Unit.BaseColor` (struct :`G` 0.314424 :`B` 1.0 :`A` 1.0) _output_get_3))
      (`/Game/Base/BP_BaseCharacter.ChangeColor` _output_get_3 "NewEnumerator1" _output_get_4))))

(fn `UserConstructionScript`
  (`parent.UserConstructionScript`))