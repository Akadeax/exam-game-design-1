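; BP_Button is a pressure button that triggers a Target actor while cubes or units stand on it.
; Begin and end overlaps with BP_Cube or BP_Unit raise and lower PressedCount, so several occupants share one press.
; The first arrival calls OnStartInteract on the Target through BI_Interactible, and the last departure calls OnEndInteract.
; The button mesh shows MI_Fire while pressed and returns to MI_Button when empty.
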(event `self.ReceiveActorBeginOverlap`
  (params (OtherActor :type "Actor Object Reference"))
  (cast `/Game/Code/BP_Cube` OtherActor
    (:`then`
      _)
    (:`CastFailed`
      (cast `/Game/Code/Characters/BP_Unit` OtherActor)))
  (`/Engine/EditorBlueprintResources/StandardMacros.IncrementInt` (`self.PressedCount`)
    (:`  `
      (`PrimitiveComponent.SetMaterial` (`self.Button`) 0 "/Game/Data/Materials/MI_Fire.MI_Fire")
      (if (== 1 (`self.PressedCount`))
        (bind _asbi_interactible (cast `/Game/Code/BI_Interactible` (`self.Target`)))
        (`/Game/Code/BI_Interactible.OnStartInteract` _asbi_interactible)))))

(event `self.ReceiveActorEndOverlap`
  (params (OtherActor :type "Actor Object Reference"))
  (cast `/Game/Code/BP_Cube` OtherActor
    (:`then`
      _)
    (:`CastFailed`
      (cast `/Game/Code/Characters/BP_Unit` OtherActor)))
  (bind _result (`/Engine/EditorBlueprintResources/StandardMacros.DecrementInt` (`self.PressedCount`))
    (:`  `
      (if (== _result 0)
        (`PrimitiveComponent.SetMaterial` (`self.Button`) 0 "/Game/Data/Materials/MI_Button.MI_Button")
        (bind _asbi_interactible (cast `/Game/Code/BI_Interactible` (`self.Target`)))
        (`/Game/Code/BI_Interactible.OnEndInteract` _asbi_interactible)))))

(fn `UserConstructionScript`)