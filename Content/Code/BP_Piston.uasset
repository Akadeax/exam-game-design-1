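; BP_Piston is an interactable piston that extends its head while an interaction is active and retracts it when the interaction ends.
; It stores the head's world position at BeginPlay as the rest point.
; The MoveT timeline plays forward on interact start and reverses on end, lerping the head from that rest point to the Target component's current world location without sweep.
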(event `self.ReceiveBeginPlay`
  (set `self.HeadBasePos` (`SceneComponent.K2_GetComponentLocation` (`self.Head`))))

(event `/Game/Code/BI_Interactible.OnStartInteract`
  (bind (_direction _time) (`Timeline|MoveT` :!label _label)
    (:`Update`
      (`SceneComponent.K2_SetWorldLocation` (`self.Head`) (`KismetMathLibrary.VLerp` (`self.HeadBasePos`) (`SceneComponent.K2_GetComponentLocation` (`self.Target`)) _time) false false))))

(event `/Game/Code/BI_Interactible.OnEndInteract`
  (goto _label :!via `Reverse`))

(fn `UserConstructionScript`)