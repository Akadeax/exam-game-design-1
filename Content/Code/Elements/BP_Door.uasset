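; BP_Door is an interactable door that slides vertically between its base position and a lowered one.
; Interaction start and end both toggle IsOpen, playing the Open timeline downward when it becomes false and reversing from the end when true.
; The timeline scales a fixed Z offset from the position cached at BeginPlay.
; BeginPlay also lowers the door if IsOpen is true, opposite to the toggle's mapping.
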(event `/Game/Code/BI_Interactible.OnStartInteract`
  (bind (_basepos_x _basepos_y _basepos_z) (`KismetMathLibrary.BreakVector` (`self.BasePos`)))
  (bind _door (`self.Door`))
  (bind (_returnvalue_x _returnvalue_y) (`KismetMathLibrary.BreakVector` (`SceneComponent.K2_GetComponentLocation` _door)))
  (bind _output_get (set `self.IsOpen` (not (`self.IsOpen`)) :!label _label))
  (switch `int` (`KismetMathLibrary.Conv_BoolToInt` _output_get)
    (:`0`
      (bind (_direction _height) (`Timeline|Open` :!label _label_2)
        (:`Update`
          (`SceneComponent.K2_SetWorldLocation` _door (`KismetMathLibrary.MakeVector` _returnvalue_x _returnvalue_y (+ (* _height -201.0) _basepos_z)) false false))))
    (:`1`
      (goto _label_2 :!via `ReverseFromEnd`))))

(event `/Game/Code/BI_Interactible.OnEndInteract`
  (goto _label))

(event `self.ReceiveBeginPlay`
  (bind (_basepos_x _basepos_y _basepos_z) (`KismetMathLibrary.BreakVector` (`self.BasePos`)))
  (set `self.BasePos` (`SceneComponent.K2_GetComponentLocation` (`self.Door`)))
  (if (`self.IsOpen`)
    (`SceneComponent.K2_SetWorldLocation` (`self.Door`) (`KismetMathLibrary.MakeVector` _basepos_x _basepos_y (- _basepos_z 201.0)) false false)))

(fn `UserConstructionScript`)