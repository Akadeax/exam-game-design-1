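; BP_Piston is a piston element that moves its Head between its starting position and a Target location.
; A timeline drives a world-space lerp without sweeping, with its play rate set from MoveTime.
; One mode extends on interact start and reverses on interact end.
; The other starts at BeginPlay and ping-pongs continuously, choosing direction by which endpoint the Head is nearer.
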(event `self.ReceiveBeginPlay`
  (bind _returnvalue (`SceneComponent.K2_GetComponentLocation` (`self.Head`)))
  (`|ExecutionSequence`
    (:`then_0`
      (set `self.HeadBasePos` (`SceneComponent.K2_GetComponentLocation` (`self.Head`))))
    (:`then_1`
      (if (`|EnumEquality` (`self.Mode`) "NewEnumerator1")
        (bind (_direction _time) (`Timeline|MoveT` :!label _label)
          (:`Update`
            (`SceneComponent.K2_SetWorldLocation` (`self.Head`) (`KismetMathLibrary.VLerp` (`self.HeadBasePos`) (`SceneComponent.K2_GetComponentLocation` (`self.Target`)) _time) false false))
          (:`Finished`
            (if (`|EnumEquality` (`self.Mode`) "NewEnumerator1")
              (if (>= (`KismetMathLibrary.Vector_Distance` (`self.HeadBasePos`) _returnvalue) (`KismetMathLibrary.Vector_Distance` _returnvalue (`SceneComponent.K2_GetComponentLocation` (`self.Target`))))
                (goto _label :!via `ReverseFromEnd`)
                (else
                  (goto _label :!via `PlayFromStart`))))))))
    (:`then_2`
      (`TimelineComponent.SetPlayRate` (`self.MoveT`) (/ 1.0 (`self.MoveTime`))))))

(event `/Game/Code/BI_Interactible.OnStartInteract`
  (if (`|EnumEquality` (`self.Mode`) "NewEnumerator0")
    (goto _label)))

(event `/Game/Code/BI_Interactible.OnEndInteract`
  (if (`|EnumEquality` (`self.Mode`) "NewEnumerator0")
    (goto _label :!via `Reverse`)))

(fn `UserConstructionScript`)