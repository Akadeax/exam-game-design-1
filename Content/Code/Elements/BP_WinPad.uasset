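; BP_WinPad is a level-exit pad that loads the next level when two units stand on it together.
; Begin and end overlap events raise and lower PlayerCount, ignoring any actor that is not a BP_Unit.
; When the count reaches two, it opens the level named by TargetLevel.
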(event `self.ReceiveActorBeginOverlap`
  (params (OtherActor :type "Actor Object Reference"))
  (cast `/Game/Code/Characters/BP_Unit` OtherActor)
  (`/Engine/EditorBlueprintResources/StandardMacros.IncrementInt` (`self.PlayerCount`)
    (:`  `
      (if (== (`self.PlayerCount`) 2)
        (`GameplayStatics.OpenLevel` (`self.TargetLevel`))))))

(event `self.ReceiveActorEndOverlap`
  (params (OtherActor :type "Actor Object Reference"))
  (cast `/Game/Code/Characters/BP_Unit` OtherActor)
  (`/Engine/EditorBlueprintResources/StandardMacros.DecrementInt` (`self.PlayerCount`)))

(fn `UserConstructionScript`)