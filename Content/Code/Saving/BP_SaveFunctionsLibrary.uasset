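; Blueprint function library that saves and restores the player's checkpoint position through a single "Checkpoint" save slot.
; SaveGame passes the player character's transform to SaveGameAtLocation, which writes a given transform into a new BP_SaveGame object and saves it to the slot.
; LoadGame reads the slot, moves the player character to the stored transform, then clears IsRespawning on BP_GameInstance.
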(fn `LoadGame`
  (bind _returnvalue (`GameplayStatics.LoadGameFromSlot` "Checkpoint"))
  (bind _asbp_save_game (cast `/Game/Code/Saving/BP_SaveGame` _returnvalue))
  (`Actor.K2_SetActorTransform` (`GameplayStatics.GetPlayerCharacter` (`local.__WorldContext`)) (`/Game/Code/Saving/BP_SaveGame.SaveTransform` _asbp_save_game) false false)
  (bind _asbp_game_instance (cast `/Game/Base/BP_GameInstance` (`GameplayStatics.GetGameInstance` (`local.__WorldContext`))))
  (set `/Game/Base/BP_GameInstance.IsRespawning` false _asbp_game_instance))

(fn `SaveGame`
  (`self.SaveGameAtLocation` (`Actor.GetTransform` (`GameplayStatics.GetPlayerCharacter` (`local.__WorldContext`)))))

(fn `SaveGameAtLocation`
  (params (Transform :type "Transform Structure"))
  (bind _returnvalue (`GameplayStatics.CreateSaveGameObject` "/Game/Code/Saving/BP_SaveGame.BP_SaveGame_C"))
  (set `/Game/Code/Saving/BP_SaveGame.SaveTransform` Transform _returnvalue)
  (`GameplayStatics.SaveGameToSlot` _returnvalue "Checkpoint"))